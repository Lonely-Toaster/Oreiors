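; HUD for the mining pod that draws a screen-centered crosshair with left and right inventory indicators and a four-step health display.
; Each DrawHUD reads health, inventory and visibility state from the player's MiningPodBlueprint character, then layers same-sized textures at one position.
; Chained integer compares pick the health texture, with none drawn outside one to four.
; Drawing requires the pod's visibility flag and HUDStart, which BeginPlay clears and HUDGameStart sets.
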(event Custom|HUDGameStart
  (Variables|Default|SetHUDStart true))

(event EventBeginPlay
  (Variables|Default|SetHUDStart false))

(event EventDrawHUD
  (params (SizeX :type Integer) (SizeY :type Integer))
  ;[1 1 1] Determine Center of Screen
  (bind _asminingpodblueprint_c (Utilities|Casting|CastToMiningPodBlueprint (Game|GetPlayerCharacter (Variables|Default|GetHUDplayerIndex))))
  (Variables|Default|SetHUDhealth (Variables|/Game/Blueprints/MiningPodBlueprint.MiningPodBlueprint_C|GetMiningPodHealth _asminingpodblueprint_c))
  (Variables|Default|SetHUDinvLeft (Variables|/Game/Blueprints/MiningPodBlueprint.MiningPodBlueprint_C|GetMiningPodInvLeft _asminingpodblueprint_c))
  (Variables|Default|SetHUDInvRight (Variables|/Game/Blueprints/MiningPodBlueprint.MiningPodBlueprint_C|GetMiningPodInvRight _asminingpodblueprint_c))
  (Variables|Default|SetHudVisible (Variables|/Game/Blueprints/MiningPodBlueprint.MiningPodBlueprint_C|GetMiningPodHUDVisible _asminingpodblueprint_c))
  (Variables|Default|SetHUDCenterX (- (/ (Math|Conversions|ToFloat(Integer) SizeX) 2.0) 128.0))
  (Variables|Default|SetHUDCenterY (- (/ (Math|Conversions|ToFloat(Integer) SizeY) 2.0) 128.0))
  ;[1 1 1] Draw HUD
  (if (Variables|Default|GetHudVisible)
    (if (Variables|Default|GetHUDStart)
      (Canvas|DrawTexture "/Game/Textures/texture_crosshair.texture_crosshair" (Variables|Default|GetHUDCenterX) (Variables|Default|GetHUDCenterY) 256.0 256.0 0.0 0.0 1.0 1.0 "(R=1.000000,G=1.000000,B=1.000000,A=1.000000)")
      ;[1 1 1] Draw HUD Inventory
      (if (Variables|Default|GetHUDinvLeft)
        (Canvas|DrawTexture "/Game/Textures/texture_ammoLeft.texture_ammoLeft" (Variables|Default|GetHUDCenterX) (Variables|Default|GetHUDCenterY) 256.0 256.0 0.0 0.0 1.0 1.0 "(R=1.000000,G=1.000000,B=1.000000,A=1.000000)"))
      (if (Variables|Default|GetHUDInvRight)
        (Canvas|DrawTexture "/Game/Textures/texture_ammoRight.texture_ammoRight" (Variables|Default|GetHUDCenterX) (Variables|Default|GetHUDCenterY) 256.0 256.0 0.0 0.0 1.0 1.0 "(R=1.000000,G=1.000000,B=1.000000,A=1.000000)"))
      ;[1 1 1] Draw HUD Health
      (Math|Integer|CompareInt (Variables|Default|GetHUDhealth) 4
        (:==
          (Canvas|DrawTexture "/Game/Textures/texture_health4.texture_health4" (Variables|Default|GetHUDCenterX) (Variables|Default|GetHUDCenterY) 256.0 256.0 0.0 0.0 1.0 1.0 "(R=1.000000,G=1.000000,B=1.000000,A=1.000000)"))
        (:<
          (Math|Integer|CompareInt (Variables|Default|GetHUDhealth) 3
            (:==
              (Canvas|DrawTexture "/Game/Textures/texture_health3.texture_health3" (Variables|Default|GetHUDCenterX) (Variables|Default|GetHUDCenterY) 256.0 256.0 0.0 0.0 1.0 1.0 "(R=1.000000,G=1.000000,B=1.000000,A=1.000000)"))
            (:<
              (Math|Integer|CompareInt (Variables|Default|GetHUDhealth) 2
                (:==
                  (Canvas|DrawTexture "/Game/Textures/texture_health2.texture_health2" (Variables|Default|GetHUDCenterX) (Variables|Default|GetHUDCenterY) 256.0 256.0 0.0 0.0 1.0 1.0 "(R=1.000000,G=1.000000,B=1.000000,A=1.000000)"))
                (:<
                  (Math|Integer|CompareInt (Variables|Default|GetHUDhealth) 1
                    (:==
                      (Canvas|DrawTexture "/Game/Textures/texture_health1.texture_health1" (Variables|Default|GetHUDCenterX) (Variables|Default|GetHUDCenterY) 256.0 256.0 0.0 0.0 1.0 1.0 "(R=1.000000,G=1.000000,B=1.000000,A=1.000000)"))))))))))))

(fn ConstructionScript)