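; Projectile actor that explodes when it hits a Character or slows nearly to a stop.
; Hits on anything other than a Character are ignored.
; Tick checks velocity length, and at or below a small threshold it starts a short Delay before detonating.
; Both paths share one sequence that spawns the explosion emitter, plays its sound and destroys the actor.
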(event EventHit
  (params (MyComp :type Primitive%20Component%20Object%20Reference) (Other :type Actor%20Object%20Reference) (OtherComp :type Primitive%20Component%20Object%20Reference) (bSelfMoved :type Boolean) (HitLocation :type Vector :default "0, 0, 0") (HitNormal :type Vector :default "0, 0, 0") (NormalImpulse :type Vector :default "0, 0, 0") (Hit :type Hit%20Result%20Structure%20%28by%20ref%29))
  (bind _returnvalue (Transformation|GetActorLocation))
  (Utilities|Casting|CastToCharacter (.HitActor (Collision|BreakHitResult Hit)))
  (Effects|SpawnEmitteratLocation "/Game/Particles/P_Explosion.P_Explosion" _returnvalue (Transformation|GetActorRotation))
  (Audio|PlaySoundatLocation "/Game/Audio/Explosion02.Explosion02" _returnvalue)
  (Actor|DestroyActor))

(event EventTick
  (params (DeltaSeconds :type Float%20%28single-precision%29))
  (bind _returnvalue (Transformation|GetActorLocation))
  (Math|Float|CompareFloat (Math|Vector|VectorLength (Transformation|GetVelocity)) 2e+01
    (:==
      _)
    (:<
      _))
  (Utilities|FlowControl|Delay 1.0)
  (Effects|SpawnEmitteratLocation "/Game/Particles/P_Explosion.P_Explosion" _returnvalue (Transformation|GetActorRotation))
  (Audio|PlaySoundatLocation "/Game/Audio/Explosion02.Explosion02" _returnvalue)
  (Actor|DestroyActor))

(fn ConstructionScript)