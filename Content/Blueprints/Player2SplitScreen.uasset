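; Starts a local split-screen mining pod session for one to four players, despite the Player2 in its name.
; SpawnPlayer1–4 set the player count and share one chain that starts the first controller and pod, then creates each additional player through nested count comparisons.
; Each pod gets an index and a game-start call.
; EnableHud then starts each MiningPodHUD in controller order, stopping at the first failed cast.
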(event Custom|SpawnPlayer1
  (bind _returnvalue (Game|GetPlayerController 0))
  (Variables|Default|SetSSPlayerCount 1)
  (Game|Feedback|ClientStopCameraShake _returnvalue "/Game/Blueprints/MainMenu_Blueprints/CameraShake.CameraShake_C")
  (bind _asminingpodplayercontroller_c (Utilities|Casting|CastToMiningPodPlayerController _returnvalue))
  (Default|ControllerGameStart _asminingpodplayercontroller_c)
  (bind _asminingpodblueprint_c (Utilities|Casting|CastToMiningPodBlueprint (Pawn|GetControlledPawn _returnvalue)))
  (Variables|/Game/Blueprints/MiningPodBlueprint.MiningPodBlueprint_C|SetMiningPodIndex _asminingpodblueprint_c 0)
  (Default|PodGameStart _asminingpodblueprint_c)
  (Math|Integer|CompareInt (Variables|Default|GetSSPlayerCount) 1
    (:>
      (bind _returnvalue_2 (Class|GameplayStatics|CreatePlayer -1))
      (Pawn|SpawnDefaultController)
      (bind _asminingpodblueprint_c_2 (Utilities|Casting|CastToMiningPodBlueprint (Pawn|GetControlledPawn _returnvalue_2)))
      (Variables|/Game/Blueprints/MiningPodBlueprint.MiningPodBlueprint_C|SetMiningPodIndex _asminingpodblueprint_c_2 1)
      (Default|PodGameStart _asminingpodblueprint_c_2)
      (Math|Integer|CompareInt (Variables|Default|GetSSPlayerCount) 2
        (:>
          (bind _returnvalue_3 (Class|GameplayStatics|CreatePlayer -1))
          (Pawn|SpawnDefaultController)
          (bind _asminingpodblueprint_c_3 (Utilities|Casting|CastToMiningPodBlueprint (Pawn|GetControlledPawn _returnvalue_3)))
          (Variables|/Game/Blueprints/MiningPodBlueprint.MiningPodBlueprint_C|SetMiningPodIndex _asminingpodblueprint_c_3 2)
          (Default|PodGameStart _asminingpodblueprint_c_3)
          (Math|Integer|CompareInt (Variables|Default|GetSSPlayerCount) 3
            (:>
              (bind _returnvalue_4 (Class|GameplayStatics|CreatePlayer -1))
              (Pawn|SpawnDefaultController)
              (bind _asminingpodblueprint_c_4 (Utilities|Casting|CastToMiningPodBlueprint (Pawn|GetControlledPawn _returnvalue_4)))
              (Variables|/Game/Blueprints/MiningPodBlueprint.MiningPodBlueprint_C|SetMiningPodIndex _asminingpodblueprint_c_4 3)
              (Default|PodGameStart _asminingpodblueprint_c_4))
            (:==
              _)))
        (:==
          _)))
    (:==
      _))
  (CallFunction|EnableHud))

(event Custom|SpawnPlayer2
  (bind _returnvalue (Game|GetPlayerController 0))
  (Variables|Default|SetSSPlayerCount 2)
  (Game|Feedback|ClientStopCameraShake _returnvalue "/Game/Blueprints/MainMenu_Blueprints/CameraShake.CameraShake_C")
  (bind _asminingpodplayercontroller_c (Utilities|Casting|CastToMiningPodPlayerController _returnvalue))
  (Default|ControllerGameStart _asminingpodplayercontroller_c)
  (bind _asminingpodblueprint_c (Utilities|Casting|CastToMiningPodBlueprint (Pawn|GetControlledPawn _returnvalue)))
  (Variables|/Game/Blueprints/MiningPodBlueprint.MiningPodBlueprint_C|SetMiningPodIndex _asminingpodblueprint_c 0)
  (Default|PodGameStart _asminingpodblueprint_c)
  (Math|Integer|CompareInt (Variables|Default|GetSSPlayerCount) 1
    (:>
      (bind _returnvalue_2 (Class|GameplayStatics|CreatePlayer -1))
      (Pawn|SpawnDefaultController)
      (bind _asminingpodblueprint_c_2 (Utilities|Casting|CastToMiningPodBlueprint (Pawn|GetControlledPawn _returnvalue_2)))
      (Variables|/Game/Blueprints/MiningPodBlueprint.MiningPodBlueprint_C|SetMiningPodIndex _asminingpodblueprint_c_2 1)
      (Default|PodGameStart _asminingpodblueprint_c_2)
      (Math|Integer|CompareInt (Variables|Default|GetSSPlayerCount) 2
        (:>
          (bind _returnvalue_3 (Class|GameplayStatics|CreatePlayer -1))
          (Pawn|SpawnDefaultController)
          (bind _asminingpodblueprint_c_3 (Utilities|Casting|CastToMiningPodBlueprint (Pawn|GetControlledPawn _returnvalue_3)))
          (Variables|/Game/Blueprints/MiningPodBlueprint.MiningPodBlueprint_C|SetMiningPodIndex _asminingpodblueprint_c_3 2)
          (Default|PodGameStart _asminingpodblueprint_c_3)
          (Math|Integer|CompareInt (Variables|Default|GetSSPlayerCount) 3
            (:>
              (bind _returnvalue_4 (Class|GameplayStatics|CreatePlayer -1))
              (Pawn|SpawnDefaultController)
              (bind _asminingpodblueprint_c_4 (Utilities|Casting|CastToMiningPodBlueprint (Pawn|GetControlledPawn _returnvalue_4)))
              (Variables|/Game/Blueprints/MiningPodBlueprint.MiningPodBlueprint_C|SetMiningPodIndex _asminingpodblueprint_c_4 3)
              (Default|PodGameStart _asminingpodblueprint_c_4))
            (:==
              _)))
        (:==
          _)))
    (:==
      _))
  (CallFunction|EnableHud))

(event Custom|SpawnPlayer3
  (bind _returnvalue (Game|GetPlayerController 0))
  (Variables|Default|SetSSPlayerCount 3)
  (Game|Feedback|ClientStopCameraShake _returnvalue "/Game/Blueprints/MainMenu_Blueprints/CameraShake.CameraShake_C")
  (bind _asminingpodplayercontroller_c (Utilities|Casting|CastToMiningPodPlayerController _returnvalue))
  (Default|ControllerGameStart _asminingpodplayercontroller_c)
  (bind _asminingpodblueprint_c (Utilities|Casting|CastToMiningPodBlueprint (Pawn|GetControlledPawn _returnvalue)))
  (Variables|/Game/Blueprints/MiningPodBlueprint.MiningPodBlueprint_C|SetMiningPodIndex _asminingpodblueprint_c 0)
  (Default|PodGameStart _asminingpodblueprint_c)
  (Math|Integer|CompareInt (Variables|Default|GetSSPlayerCount) 1
    (:>
      (bind _returnvalue_2 (Class|GameplayStatics|CreatePlayer -1))
      (Pawn|SpawnDefaultController)
      (bind _asminingpodblueprint_c_2 (Utilities|Casting|CastToMiningPodBlueprint (Pawn|GetControlledPawn _returnvalue_2)))
      (Variables|/Game/Blueprints/MiningPodBlueprint.MiningPodBlueprint_C|SetMiningPodIndex _asminingpodblueprint_c_2 1)
      (Default|PodGameStart _asminingpodblueprint_c_2)
      (Math|Integer|CompareInt (Variables|Default|GetSSPlayerCount) 2
        (:>
          (bind _returnvalue_3 (Class|GameplayStatics|CreatePlayer -1))
          (Pawn|SpawnDefaultController)
          (bind _asminingpodblueprint_c_3 (Utilities|Casting|CastToMiningPodBlueprint (Pawn|GetControlledPawn _returnvalue_3)))
          (Variables|/Game/Blueprints/MiningPodBlueprint.MiningPodBlueprint_C|SetMiningPodIndex _asminingpodblueprint_c_3 2)
          (Default|PodGameStart _asminingpodblueprint_c_3)
          (Math|Integer|CompareInt (Variables|Default|GetSSPlayerCount) 3
            (:>
              (bind _returnvalue_4 (Class|GameplayStatics|CreatePlayer -1))
              (Pawn|SpawnDefaultController)
              (bind _asminingpodblueprint_c_4 (Utilities|Casting|CastToMiningPodBlueprint (Pawn|GetControlledPawn _returnvalue_4)))
              (Variables|/Game/Blueprints/MiningPodBlueprint.MiningPodBlueprint_C|SetMiningPodIndex _asminingpodblueprint_c_4 3)
              (Default|PodGameStart _asminingpodblueprint_c_4))
            (:==
              _)))
        (:==
          _)))
    (:==
      _))
  (CallFunction|EnableHud))

(event Custom|SpawnPlayer4
  (bind _returnvalue (Game|GetPlayerController 0))
  (Variables|Default|SetSSPlayerCount 4)
  (Game|Feedback|ClientStopCameraShake _returnvalue "/Game/Blueprints/MainMenu_Blueprints/CameraShake.CameraShake_C")
  (bind _asminingpodplayercontroller_c (Utilities|Casting|CastToMiningPodPlayerController _returnvalue))
  (Default|ControllerGameStart _asminingpodplayercontroller_c)
  (bind _asminingpodblueprint_c (Utilities|Casting|CastToMiningPodBlueprint (Pawn|GetControlledPawn _returnvalue)))
  (Variables|/Game/Blueprints/MiningPodBlueprint.MiningPodBlueprint_C|SetMiningPodIndex _asminingpodblueprint_c 0)
  (Default|PodGameStart _asminingpodblueprint_c)
  (Math|Integer|CompareInt (Variables|Default|GetSSPlayerCount) 1
    (:>
      (bind _returnvalue_2 (Class|GameplayStatics|CreatePlayer -1))
      (Pawn|SpawnDefaultController)
      (bind _asminingpodblueprint_c_2 (Utilities|Casting|CastToMiningPodBlueprint (Pawn|GetControlledPawn _returnvalue_2)))
      (Variables|/Game/Blueprints/MiningPodBlueprint.MiningPodBlueprint_C|SetMiningPodIndex _asminingpodblueprint_c_2 1)
      (Default|PodGameStart _asminingpodblueprint_c_2)
      (Math|Integer|CompareInt (Variables|Default|GetSSPlayerCount) 2
        (:>
          (bind _returnvalue_3 (Class|GameplayStatics|CreatePlayer -1))
          (Pawn|SpawnDefaultController)
          (bind _asminingpodblueprint_c_3 (Utilities|Casting|CastToMiningPodBlueprint (Pawn|GetControlledPawn _returnvalue_3)))
          (Variables|/Game/Blueprints/MiningPodBlueprint.MiningPodBlueprint_C|SetMiningPodIndex _asminingpodblueprint_c_3 2)
          (Default|PodGameStart _asminingpodblueprint_c_3)
          (Math|Integer|CompareInt (Variables|Default|GetSSPlayerCount) 3
            (:>
              (bind _returnvalue_4 (Class|GameplayStatics|CreatePlayer -1))
              (Pawn|SpawnDefaultController)
              (bind _asminingpodblueprint_c_4 (Utilities|Casting|CastToMiningPodBlueprint (Pawn|GetControlledPawn _returnvalue_4)))
              (Variables|/Game/Blueprints/MiningPodBlueprint.MiningPodBlueprint_C|SetMiningPodIndex _asminingpodblueprint_c_4 3)
              (Default|PodGameStart _asminingpodblueprint_c_4))
            (:==
              _)))
        (:==
          _)))
    (:==
      _))
  (CallFunction|EnableHud))

(fn ConstructionScript)

(fn EnableHud
  (bind _asminingpodhud_c (Utilities|Casting|CastToMiningPodHUD (HUD|GetHUD (Game|GetPlayerController 0))))
  (Default|HUDGameStart _asminingpodhud_c)
  (bind _asminingpodhud_c_2 (Utilities|Casting|CastToMiningPodHUD (HUD|GetHUD (Game|GetPlayerController 1))))
  (Default|HUDGameStart _asminingpodhud_c_2)
  (bind _asminingpodhud_c_3 (Utilities|Casting|CastToMiningPodHUD (HUD|GetHUD (Game|GetPlayerController 2))))
  (Default|HUDGameStart _asminingpodhud_c_3)
  (bind _asminingpodhud_c_4 (Utilities|Casting|CastToMiningPodHUD (HUD|GetHUD (Game|GetPlayerController 3))))
  (Default|HUDGameStart _asminingpodhud_c_4))