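; HUD Blueprint that draws a screen-centered crosshair with ammo and health indicators.
; On each DrawHUD, if HUDIsDrawn is set, it layers equally sized, centered textures: the crosshair, then left and right ammo overlays gated by the HUDInvLeft and HUDInvRight flags.
; A nested integer-compare chain on HUDHealth picks one of four health textures, drawing none for values outside one to four.
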(event EventDrawHUD
  (params (SizeX :type Integer) (SizeY :type Integer))
  (Variables|Default|SetCenterX (- (/ (Math|Conversions|ToFloat(Integer) SizeX) 2.0) 128.0))
  (Variables|Default|SetCenterY (- (/ (Math|Conversions|ToFloat(Integer) SizeY) 2.0) 128.0))
  (if (Variables|Default|GetHUD_is_drawn)
    (Canvas|DrawTexture "/Game/Textures/texture_crosshair.texture_crosshair" (Variables|Default|GetCenterX) (Variables|Default|GetCenterY) 256.0 256.0 0.0 0.0 1.0 1.0 "(R=1.000000,G=1.000000,B=1.000000,A=1.000000)")
    (if (Variables|Default|GetHUD_inv_left)
      (Canvas|DrawTexture "/Game/Textures/texture_ammoLeft.texture_ammoLeft" (Variables|Default|GetCenterX) (Variables|Default|GetCenterY) 256.0 256.0 0.0 0.0 1.0 1.0 "(R=1.000000,G=1.000000,B=1.000000,A=1.000000)"))
    (if (Variables|Default|GetHUD_inv_right)
      (Canvas|DrawTexture "/Game/Textures/texture_ammoRight.texture_ammoRight" (Variables|Default|GetCenterX) (Variables|Default|GetCenterY) 256.0 256.0 0.0 0.0 1.0 1.0 "(R=1.000000,G=1.000000,B=1.000000,A=1.000000)"))
    (Math|Integer|CompareInt (Variables|Default|GetHUD_health) 4
      (:==
        (Canvas|DrawTexture "/Game/Textures/texture_health4.texture_health4" (Variables|Default|GetCenterX) (Variables|Default|GetCenterY) 256.0 256.0 0.0 0.0 1.0 1.0 "(R=1.000000,G=1.000000,B=1.000000,A=1.000000)"))
      (:<
        (Math|Integer|CompareInt (Variables|Default|GetHUD_health) 3
          (:==
            (Canvas|DrawTexture "/Game/Textures/texture_health3.texture_health3" (Variables|Default|GetCenterX) (Variables|Default|GetCenterY) 256.0 256.0 0.0 0.0 1.0 1.0 "(R=1.000000,G=1.000000,B=1.000000,A=1.000000)"))
          (:<
            (Math|Integer|CompareInt (Variables|Default|GetHUD_health) 2
              (:==
                (Canvas|DrawTexture "/Game/Textures/texture_health2.texture_health2" (Variables|Default|GetCenterX) (Variables|Default|GetCenterY) 256.0 256.0 0.0 0.0 1.0 1.0 "(R=1.000000,G=1.000000,B=1.000000,A=1.000000)"))
              (:<
                (Math|Integer|CompareInt (Variables|Default|GetHUD_health) 1
                  (:==
                    (Canvas|DrawTexture "/Game/Textures/texture_health1.texture_health1" (Variables|Default|GetCenterX) (Variables|Default|GetCenterY) 256.0 256.0 0.0 0.0 1.0 1.0 "(R=1.000000,G=1.000000,B=1.000000,A=1.000000)")))))))))))

(fn ConstructionScript)