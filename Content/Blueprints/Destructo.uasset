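; Destructo is a destructible actor that loses health when hit by a projectile and explodes when it runs out.
; Its Hit event casts the hit result's actor to Projectile, ignores anything else, and subtracts a fixed amount from Health.
; At zero or below, it spawns an explosion emitter and sound at its location, then destroys itself.
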(event EventHit
  (params (MyComp :type Primitive%20Component%20Object%20Reference) (Other :type Actor%20Object%20Reference) (OtherComp :type Primitive%20Component%20Object%20Reference) (bSelfMoved :type Boolean) (HitLocation :type Vector :default "0, 0, 0") (HitNormal :type Vector :default "0, 0, 0") (NormalImpulse :type Vector :default "0, 0, 0") (Hit :type Hit%20Result%20Structure%20%28by%20ref%29))
  (bind _returnvalue (Transformation|GetActorLocation))
  (Utilities|Casting|CastToProjectile (.HitActor (Collision|BreakHitResult Hit)))
  (Variables|Default|Sethealth (- (Variables|Default|Gethealth) 5))
  (Math|Integer|CompareInt (Variables|Default|Gethealth) 0
    (:==
      _)
    (:<
      _))
  (Effects|SpawnEmitteratLocation "/Game/Particles/P_Explosion.P_Explosion" _returnvalue (Transformation|GetActorRotation))
  (Audio|PlaySoundatLocation "/Game/Audio/Explosion02.Explosion02" _returnvalue)
  (Actor|DestroyActor))

(fn ConstructionScript)