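; Player selection submenu of the main menu, built from clickable components and text, with a 1 Players button and a Back button.
; The 1 Players button opens levelCrater, while Back calls the PlayerBackButtonClicked dispatcher and resets its text material.
; Hovering swaps the text to a mouse-over material and plays a click sound, then restores it when the cursor leaves.
; All button events are gated by IsActive.
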(event OnClicked(Button_1)
  (params (TouchedComponent :type Primitive%20Component%20Object%20Reference))
  ;[1 1 1] 1 Players Button
  (if (Variables|Default|GetIsActive)
    (Game|OpenLevel(byName) "levelCrater")))

(event OnBeginCursorOver(Button_1)
  (params (TouchedComponent :type Primitive%20Component%20Object%20Reference))
  (bind _text_1 (Variables|Default|GetText_1))
  ;[1 1 1] 1 Players Button
  (if (Variables|Default|GetIsActive)
    (Rendering|Material|SetMaterial _text_1 0 "/Game/Materials/TextMaterial_MainMenu_MouseOver.TextMaterial_MainMenu_MouseOver")
    (Class|GameplayStatics|PlaySoundAttached "/Game/Audio/Click_04.Click_04" _text_1)))

(event OnEndCursorOver(Button_1)
  (params (TouchedComponent :type Primitive%20Component%20Object%20Reference))
  ;[1 1 1] 1 Players Button
  (if (Variables|Default|GetIsActive)
    (Rendering|Material|SetMaterial (Variables|Default|GetText_1) 0 "/Game/Materials/TextMaterial_MainMenu.TextMaterial_MainMenu")))

(event OnBeginCursorOver(Button_Back)
  (params (TouchedComponent :type Primitive%20Component%20Object%20Reference))
  (bind _text_back (Variables|Default|GetText_Back))
  ;[1 1 1] Back Button
  (if (Variables|Default|GetIsActive)
    (Rendering|Material|SetMaterial _text_back 0 "/Game/Materials/TextMaterial_MainMenu_MouseOver.TextMaterial_MainMenu_MouseOver")
    (Class|GameplayStatics|PlaySoundAttached "/Game/Audio/Click_04.Click_04" _text_back)))

(event OnEndCursorOver(Button_Back)
  (params (TouchedComponent :type Primitive%20Component%20Object%20Reference))
  ;[1 1 1] Back Button
  (if (Variables|Default|GetIsActive)
    (Rendering|Material|SetMaterial (Variables|Default|GetText_Back) 0 "/Game/Materials/TextMaterial_MainMenu.TextMaterial_MainMenu")))

(event OnClicked(Button_Back)
  (params (TouchedComponent :type Primitive%20Component%20Object%20Reference))
  ;[1 1 1] Back Button
  (if (Variables|Default|GetIsActive)
    (Default|CallPlayerBackButtonClicked)
    (Rendering|Material|SetMaterial (Variables|Default|GetText_Back) 0 "/Game/Materials/TextMaterial_MainMenu.TextMaterial_MainMenu")))

(fn ConstructionScript)