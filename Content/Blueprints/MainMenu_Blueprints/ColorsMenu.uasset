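; Main menu colour picker where the four players each choose a colour for their pod from clickable swatches.
; While the menu is active, a swatch click passes ColorTest, which rejects any colour a pod already holds, then stores that pod's colour.
; ColorChanging writes the matching RGB to the pod's vector parameter in the PodColors Material Parameter Collection.
; The Back button fires CallColorsBackButtonClicked and swaps its text material on hover, with a sound.
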(event OnClicked(Player2_Blue)
  (params (TouchedComponent :type Primitive%20Component%20Object%20Reference))
  ;[1 1 1] Pod 2 Color
  (if (Variables|Default|GetIsActive)
    (bind _test (CallFunction|ColorTest "blue"))
    (if _test
      (Variables|Default|SetPod2Color "blue")
      (CallFunction|ColorChanging (Variables|Default|GetPod2) (Variables|Default|GetPod2Color)))))

(event OnClicked(Player2_Red)
  (params (TouchedComponent :type Primitive%20Component%20Object%20Reference))
  ;[1 1 1] Pod 2 Color
  (if (Variables|Default|GetIsActive)
    (bind _test (CallFunction|ColorTest "red"))
    (if _test
      (Variables|Default|SetPod2Color "red")
      (CallFunction|ColorChanging (Variables|Default|GetPod2) (Variables|Default|GetPod2Color)))))

(event OnClicked(Player2_Yellow)
  (params (TouchedComponent :type Primitive%20Component%20Object%20Reference))
  ;[1 1 1] Pod 2 Color
  (if (Variables|Default|GetIsActive)
    (bind _test (CallFunction|ColorTest "yellow"))
    (if _test
      (Variables|Default|SetPod2Color "yellow")
      (CallFunction|ColorChanging (Variables|Default|GetPod2) (Variables|Default|GetPod2Color)))))

(event OnClicked(Player2_Green)
  (params (TouchedComponent :type Primitive%20Component%20Object%20Reference))
  ;[1 1 1] Pod 2 Color
  (if (Variables|Default|GetIsActive)
    (bind _test (CallFunction|ColorTest "green"))
    (if _test
      (Variables|Default|SetPod2Color "green")
      (CallFunction|ColorChanging (Variables|Default|GetPod2) (Variables|Default|GetPod2Color)))))

(event OnClicked(Player2_Pink)
  (params (TouchedComponent :type Primitive%20Component%20Object%20Reference))
  ;[1 1 1] Pod 2 Color
  (if (Variables|Default|GetIsActive)
    (bind _test (CallFunction|ColorTest "pink"))
    (if _test
      (Variables|Default|SetPod2Color "pink")
      (CallFunction|ColorChanging (Variables|Default|GetPod2) (Variables|Default|GetPod2Color)))))

(event OnClicked(Player2_Orange)
  (params (TouchedComponent :type Primitive%20Component%20Object%20Reference))
  ;[1 1 1] Pod 2 Color
  (if (Variables|Default|GetIsActive)
    (bind _test (CallFunction|ColorTest "orange"))
    (if _test
      (Variables|Default|SetPod2Color "orange")
      (CallFunction|ColorChanging (Variables|Default|GetPod2) (Variables|Default|GetPod2Color)))))

(event OnClicked(Player2_Purple)
  (params (TouchedComponent :type Primitive%20Component%20Object%20Reference))
  ;[1 1 1] Pod 2 Color
  (if (Variables|Default|GetIsActive)
    (bind _test (CallFunction|ColorTest "purple"))
    (if _test
      (Variables|Default|SetPod2Color "purple")
      (CallFunction|ColorChanging (Variables|Default|GetPod2) (Variables|Default|GetPod2Color)))))

(event OnClicked(Player2_White)
  (params (TouchedComponent :type Primitive%20Component%20Object%20Reference))
  ;[1 1 1] Pod 2 Color
  (if (Variables|Default|GetIsActive)
    (bind _test (CallFunction|ColorTest "white"))
    (if _test
      (Variables|Default|SetPod2Color "white")
      (CallFunction|ColorChanging (Variables|Default|GetPod2) (Variables|Default|GetPod2Color)))))

(event OnClicked(Player2_Black)
  (params (TouchedComponent :type Primitive%20Component%20Object%20Reference))
  ;[1 1 1] Pod 2 Color
  (if (Variables|Default|GetIsActive)
    (bind _test (CallFunction|ColorTest "black"))
    (if _test
      (Variables|Default|SetPod2Color "black")
      (CallFunction|ColorChanging (Variables|Default|GetPod2) (Variables|Default|GetPod2Color)))))

(event OnClicked(Button_Back)
  (params (TouchedComponent :type Primitive%20Component%20Object%20Reference))
  ;[1 1 1] Back Button
  (if (Variables|Default|GetIsActive)
    (Default|CallColorsBackButtonClicked)
    (Rendering|Material|SetMaterial (Variables|Default|GetText_Back) 0 "/Game/Materials/TextMaterial_MainMenu.TextMaterial_MainMenu")))

(event OnClicked(Player3_Blue)
  (params (TouchedComponent :type Primitive%20Component%20Object%20Reference))
  ;[1 1 1] Pod 3 Color
  (if (Variables|Default|GetIsActive)
    (bind _test (CallFunction|ColorTest "blue"))
    (if _test
      (Variables|Default|SetPod3Color "blue")
      (CallFunction|ColorChanging (Variables|Default|GetPod3) (Variables|Default|GetPod3Color)))))

(event OnClicked(Player3_Red)
  (params (TouchedComponent :type Primitive%20Component%20Object%20Reference))
  ;[1 1 1] Pod 3 Color
  (if (Variables|Default|GetIsActive)
    (bind _test (CallFunction|ColorTest "red"))
    (if _test
      (Variables|Default|SetPod3Color "red")
      (CallFunction|ColorChanging (Variables|Default|GetPod3) (Variables|Default|GetPod3Color)))))

(event OnBeginCursorOver(Button_Back)
  (params (TouchedComponent :type Primitive%20Component%20Object%20Reference))
  (bind _text_back (Variables|Default|GetText_Back))
  ;[1 1 1] Back Button
  (if (Variables|Default|GetIsActive)
    (Rendering|Material|SetMaterial _text_back 0 "/Game/Materials/TextMaterial_MainMenu_MouseOver.TextMaterial_MainMenu_MouseOver")
    (Class|GameplayStatics|PlaySoundAttached "/Game/Audio/Click_04.Click_04" _text_back)))

(event OnClicked(Player3_Yellow)
  (params (TouchedComponent :type Primitive%20Component%20Object%20Reference))
  ;[1 1 1] Pod 3 Color
  (if (Variables|Default|GetIsActive)
    (bind _test (CallFunction|ColorTest "yellow"))
    (if _test
      (Variables|Default|SetPod3Color "yellow")
      (CallFunction|ColorChanging (Variables|Default|GetPod3) (Variables|Default|GetPod3Color)))))

(event OnClicked(Player3_Green)
  (params (TouchedComponent :type Primitive%20Component%20Object%20Reference))
  ;[1 1 1] Pod 3 Color
  (if (Variables|Default|GetIsActive)
    (bind _test (CallFunction|ColorTest "green"))
    (if _test
      (Variables|Default|SetPod3Color "green")
      (CallFunction|ColorChanging (Variables|Default|GetPod3) (Variables|Default|GetPod3Color)))))

(event OnClicked(Player3_Pink)
  (params (TouchedComponent :type Primitive%20Component%20Object%20Reference))
  ;[1 1 1] Pod 3 Color
  (if (Variables|Default|GetIsActive)
    (bind _test (CallFunction|ColorTest "pink"))
    (if _test
      (Variables|Default|SetPod3Color "pink")
      (CallFunction|ColorChanging (Variables|Default|GetPod3) (Variables|Default|GetPod3Color)))))

(event OnEndCursorOver(Button_Back)
  (params (TouchedComponent :type Primitive%20Component%20Object%20Reference))
  ;[1 1 1] Back Button
  (if (Variables|Default|GetIsActive)
    (Rendering|Material|SetMaterial (Variables|Default|GetText_Back) 0 "/Game/Materials/TextMaterial_MainMenu.TextMaterial_MainMenu")))

(event OnClicked(Player3_Orange)
  (params (TouchedComponent :type Primitive%20Component%20Object%20Reference))
  ;[1 1 1] Pod 3 Color
  (if (Variables|Default|GetIsActive)
    (bind _test (CallFunction|ColorTest "orange"))
    (if _test
      (Variables|Default|SetPod3Color "orange")
      (CallFunction|ColorChanging (Variables|Default|GetPod3) (Variables|Default|GetPod3Color)))))

(event OnClicked(Player3_Purple)
  (params (TouchedComponent :type Primitive%20Component%20Object%20Reference))
  ;[1 1 1] Pod 3 Color
  (if (Variables|Default|GetIsActive)
    (bind _test (CallFunction|ColorTest "purple"))
    (if _test
      (Variables|Default|SetPod3Color "purple")
      (CallFunction|ColorChanging (Variables|Default|GetPod3) (Variables|Default|GetPod3Color)))))

(event OnClicked(Player3_White)
  (params (TouchedComponent :type Primitive%20Component%20Object%20Reference))
  ;[1 1 1] Pod 3 Color
  (if (Variables|Default|GetIsActive)
    (bind _test (CallFunction|ColorTest "white"))
    (if _test
      (Variables|Default|SetPod3Color "white")
      (CallFunction|ColorChanging (Variables|Default|GetPod3) (Variables|Default|GetPod3Color)))))

(event OnClicked(Player3_Black)
  (params (TouchedComponent :type Primitive%20Component%20Object%20Reference))
  ;[1 1 1] Pod 3 Color
  (if (Variables|Default|GetIsActive)
    (bind _test (CallFunction|ColorTest "black"))
    (if _test
      (Variables|Default|SetPod3Color "black")
      (CallFunction|ColorChanging (Variables|Default|GetPod3) (Variables|Default|GetPod3Color)))))

(event OnClicked(Player1_Blue)
  (params (TouchedComponent :type Primitive%20Component%20Object%20Reference))
  ;[1 1 1] Pod 1 Color
  (if (Variables|Default|GetIsActive)
    (bind _test (CallFunction|ColorTest "blue"))
    (if _test
      (Variables|Default|SetPod1Color "blue")
      (CallFunction|ColorChanging (Variables|Default|GetPod1) (Variables|Default|GetPod1Color)))))

(event OnClicked(Player1_Red)
  (params (TouchedComponent :type Primitive%20Component%20Object%20Reference))
  ;[1 1 1] Pod 1 Color
  (if (Variables|Default|GetIsActive)
    (bind _test (CallFunction|ColorTest "red"))
    (if _test
      (Variables|Default|SetPod1Color "red")
      (CallFunction|ColorChanging (Variables|Default|GetPod1) (Variables|Default|GetPod1Color)))))

(event OnClicked(Player1_Green)
  (params (TouchedComponent :type Primitive%20Component%20Object%20Reference))
  ;[1 1 1] Pod 1 Color
  (if (Variables|Default|GetIsActive)
    (bind _test (CallFunction|ColorTest "green"))
    (if _test
      (Variables|Default|SetPod1Color "green")
      (CallFunction|ColorChanging (Variables|Default|GetPod1) (Variables|Default|GetPod1Color)))))

(event OnClicked(Player1_Pink)
  (params (TouchedComponent :type Primitive%20Component%20Object%20Reference))
  ;[1 1 1] Pod 1 Color
  (if (Variables|Default|GetIsActive)
    (bind _test (CallFunction|ColorTest "pink"))
    (if _test
      (Variables|Default|SetPod1Color "pink")
      (CallFunction|ColorChanging (Variables|Default|GetPod1) (Variables|Default|GetPod1Color)))))

(event OnClicked(Player1_Yellow)
  (params (TouchedComponent :type Primitive%20Component%20Object%20Reference))
  ;[1 1 1] Pod 1 Color
  (if (Variables|Default|GetIsActive)
    (bind _test (CallFunction|ColorTest "yellow"))
    (if _test
      (Variables|Default|SetPod1Color "yellow")
      (CallFunction|ColorChanging (Variables|Default|GetPod1) (Variables|Default|GetPod1Color)))))

(event OnClicked(Player1_Orange)
  (params (TouchedComponent :type Primitive%20Component%20Object%20Reference))
  ;[1 1 1] Pod 1 Color
  (if (Variables|Default|GetIsActive)
    (bind _test (CallFunction|ColorTest "orange"))
    (if _test
      (Variables|Default|SetPod1Color "orange")
      (CallFunction|ColorChanging (Variables|Default|GetPod1) (Variables|Default|GetPod1Color)))))

(event OnClicked(Player1_Purple)
  (params (TouchedComponent :type Primitive%20Component%20Object%20Reference))
  ;[1 1 1] Pod 1 Color
  (if (Variables|Default|GetIsActive)
    (bind _test (CallFunction|ColorTest "purple"))
    (if _test
      (Variables|Default|SetPod1Color "purple")
      (CallFunction|ColorChanging (Variables|Default|GetPod1) (Variables|Default|GetPod1Color)))))

(event OnClicked(Player1_White)
  (params (TouchedComponent :type Primitive%20Component%20Object%20Reference))
  ;[1 1 1] Pod 1 Color
  (if (Variables|Default|GetIsActive)
    (bind _test (CallFunction|ColorTest "white"))
    (if _test
      (Variables|Default|SetPod1Color "white")
      (CallFunction|ColorChanging (Variables|Default|GetPod1) (Variables|Default|GetPod1Color)))))

(event OnClicked(Player1_Black)
  (params (TouchedComponent :type Primitive%20Component%20Object%20Reference))
  ;[1 1 1] Pod 1 Color
  (if (Variables|Default|GetIsActive)
    (bind _test (CallFunction|ColorTest "black"))
    (if _test
      (Variables|Default|SetPod1Color "black")
      (CallFunction|ColorChanging (Variables|Default|GetPod1) (Variables|Default|GetPod1Color)))))

(event OnClicked(Player4_Blue)
  (params (TouchedComponent :type Primitive%20Component%20Object%20Reference))
  ;[1 1 1] Pod 4 Color
  (if (Variables|Default|GetIsActive)
    (bind _test (CallFunction|ColorTest "blue"))
    (if _test
      (Variables|Default|SetPod4Color "blue")
      (CallFunction|ColorChanging (Variables|Default|GetPod4) (Variables|Default|GetPod4Color)))))

(event OnClicked(Player4_Red)
  (params (TouchedComponent :type Primitive%20Component%20Object%20Reference))
  ;[1 1 1] Pod 4 Color
  (if (Variables|Default|GetIsActive)
    (bind _test (CallFunction|ColorTest "red"))
    (if _test
      (Variables|Default|SetPod4Color "red")
      (CallFunction|ColorChanging (Variables|Default|GetPod4) (Variables|Default|GetPod4Color)))))

(event OnClicked(Player4_Yellow)
  (params (TouchedComponent :type Primitive%20Component%20Object%20Reference))
  ;[1 1 1] Pod 4 Color
  (if (Variables|Default|GetIsActive)
    (bind _test (CallFunction|ColorTest "yellow"))
    (if _test
      (Variables|Default|SetPod4Color "yellow")
      (CallFunction|ColorChanging (Variables|Default|GetPod4) (Variables|Default|GetPod4Color)))))

(event OnClicked(Player4_Green)
  (params (TouchedComponent :type Primitive%20Component%20Object%20Reference))
  ;[1 1 1] Pod 4 Color
  (if (Variables|Default|GetIsActive)
    (bind _test (CallFunction|ColorTest "green"))
    (if _test
      (Variables|Default|SetPod4Color "green")
      (CallFunction|ColorChanging (Variables|Default|GetPod4) (Variables|Default|GetPod4Color)))))

(event OnClicked(Player4_Pink)
  (params (TouchedComponent :type Primitive%20Component%20Object%20Reference))
  ;[1 1 1] Pod 4 Color
  (if (Variables|Default|GetIsActive)
    (bind _test (CallFunction|ColorTest "pink"))
    (if _test
      (Variables|Default|SetPod4Color "pink")
      (CallFunction|ColorChanging (Variables|Default|GetPod4) (Variables|Default|GetPod4Color)))))

(event OnClicked(Player4_Orange)
  (params (TouchedComponent :type Primitive%20Component%20Object%20Reference))
  ;[1 1 1] Pod 4 Color
  (if (Variables|Default|GetIsActive)
    (bind _test (CallFunction|ColorTest "orange"))
    (if _test
      (Variables|Default|SetPod4Color "orange")
      (CallFunction|ColorChanging (Variables|Default|GetPod4) (Variables|Default|GetPod4Color)))))

(event OnClicked(Player4_Purple)
  (params (TouchedComponent :type Primitive%20Component%20Object%20Reference))
  ;[1 1 1] Pod 4 Color
  (if (Variables|Default|GetIsActive)
    (bind _test (CallFunction|ColorTest "purple"))
    (if _test
      (Variables|Default|SetPod4Color "purple")
      (CallFunction|ColorChanging (Variables|Default|GetPod4) (Variables|Default|GetPod4Color)))))

(event OnClicked(Player4_White)
  (params (TouchedComponent :type Primitive%20Component%20Object%20Reference))
  ;[1 1 1] Pod 4 Color
  (if (Variables|Default|GetIsActive)
    (bind _test (CallFunction|ColorTest "white"))
    (if _test
      (Variables|Default|SetPod4Color "white")
      (CallFunction|ColorChanging (Variables|Default|GetPod4) (Variables|Default|GetPod4Color)))))

(event OnClicked(Player4_Black)
  (params (TouchedComponent :type Primitive%20Component%20Object%20Reference))
  ;[1 1 1] Pod 4 Color
  (if (Variables|Default|GetIsActive)
    (bind _test (CallFunction|ColorTest "black"))
    (if _test
      (Variables|Default|SetPod4Color "black")
      (CallFunction|ColorChanging (Variables|Default|GetPod4) (Variables|Default|GetPod4Color)))))

(fn ConstructionScript)

(fn ColorTest
  (params (color :type String))
  (if (Utilities|Enum|NotEqual(Enum) (Variables|Default|GetPod1Color) color)
    (if (Utilities|Enum|NotEqual(Enum) (Variables|Default|GetPod2Color) color)
      (if (Utilities|Enum|NotEqual(Enum) (Variables|Default|GetPod3Color) color)
        (if (Utilities|Enum|NotEqual(Enum) (Variables|Default|GetPod4Color) color)
          (return true))))))

(fn ColorChanging
  (params (PodName :type Name :default "None") (PodColor :type String))
  (switch string PodColor
    (:blue
      ;[1 1 1] Blue
      (Rendering|Material|SetVectorParameterValue "/Game/Materials/PodColors.PodColors" PodName (Utilities|Struct|MakeLinearColor 0.0 0.2 1.0 0.0) :!class /Script/Engine.KismetMaterialLibrary))
    (:red
      ;[1 1 1] Red
      (Rendering|Material|SetVectorParameterValue "/Game/Materials/PodColors.PodColors" PodName (Utilities|Struct|MakeLinearColor 1.0 0.0 0.0 0.0) :!class /Script/Engine.KismetMaterialLibrary))
    (:yellow
      ;[1 1 1] Yellow
      (Rendering|Material|SetVectorParameterValue "/Game/Materials/PodColors.PodColors" PodName (Utilities|Struct|MakeLinearColor 0.9 0.9 0.0 0.0) :!class /Script/Engine.KismetMaterialLibrary))
    (:green
      ;[1 1 1] Green
      (Rendering|Material|SetVectorParameterValue "/Game/Materials/PodColors.PodColors" PodName (Utilities|Struct|MakeLinearColor 0.0 1.0 0.1 0.0) :!class /Script/Engine.KismetMaterialLibrary))
    (:pink
      ;[1 1 1] Pink
      (Rendering|Material|SetVectorParameterValue "/Game/Materials/PodColors.PodColors" PodName (Utilities|Struct|MakeLinearColor 1.0 0.3 0.5 0.0) :!class /Script/Engine.KismetMaterialLibrary))
    (:orange
      ;[1 1 1] Orange
      (Rendering|Material|SetVectorParameterValue "/Game/Materials/PodColors.PodColors" PodName (Utilities|Struct|MakeLinearColor 0.7 0.3 0.0 0.0) :!class /Script/Engine.KismetMaterialLibrary))
    (:purple
      ;[1 1 1] Purple
      (Rendering|Material|SetVectorParameterValue "/Game/Materials/PodColors.PodColors" PodName (Utilities|Struct|MakeLinearColor 0.3 0.0 0.4 0.0) :!class /Script/Engine.KismetMaterialLibrary))
    (:white
      ;[1 1 1] White
      (Rendering|Material|SetVectorParameterValue "/Game/Materials/PodColors.PodColors" PodName (Utilities|Struct|MakeLinearColor 0.6 0.6 0.6 0.0) :!class /Script/Engine.KismetMaterialLibrary))
    (:black
      ;[1 1 1] Black
      (Rendering|Material|SetVectorParameterValue "/Game/Materials/PodColors.PodColors" PodName (Utilities|Struct|MakeLinearColor 0.0 0.0 0.0 0.0) :!class /Script/Engine.KismetMaterialLibrary))))