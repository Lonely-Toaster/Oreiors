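; StartMenu is an in-world main menu actor with Play, Options and Quit buttons built from clickable components and text.
; While IsActive is set, hovering a button swaps its text to a highlight material and plays a click sound, and leaving or clicking restores the normal material.
; Play and Options clicks fire event dispatchers for external listeners, while Quit exits the game directly.
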(event OnClicked(Button_Quit)
  (params (TouchedComponent :type Primitive%20Component%20Object%20Reference))
  ;[1 1 1] Quit Button
  (if (Variables|Default|GetIsActive)
    (Game|QuitGame)
    (Rendering|Material|SetMaterial (Variables|Default|GetText_Quit) 0 "/Game/Materials/TextMaterial_MainMenu.TextMaterial_MainMenu")))

(event OnBeginCursorOver(Button_Play)
  (params (TouchedComponent :type Primitive%20Component%20Object%20Reference))
  (bind _text_play (Variables|Default|GetText_Play))
  ;[1 1 1] Play Button
  (if (Variables|Default|GetIsActive)
    (Rendering|Material|SetMaterial _text_play 0 "/Game/Materials/TextMaterial_MainMenu_MouseOver.TextMaterial_MainMenu_MouseOver")
    (Class|GameplayStatics|PlaySoundAttached "/Game/Audio/Click_04.Click_04" _text_play)))

(event OnEndCursorOver(Button_Play)
  (params (TouchedComponent :type Primitive%20Component%20Object%20Reference))
  ;[1 1 1] Play Button
  (if (Variables|Default|GetIsActive)
    (Rendering|Material|SetMaterial (Variables|Default|GetText_Play) 0 "/Game/Materials/TextMaterial_MainMenu.TextMaterial_MainMenu")))

(event OnBeginCursorOver(Button_Quit)
  (params (TouchedComponent :type Primitive%20Component%20Object%20Reference))
  (bind _text_quit (Variables|Default|GetText_Quit))
  ;[1 1 1] Quit Button
  (if (Variables|Default|GetIsActive)
    (Rendering|Material|SetMaterial _text_quit 0 "/Game/Materials/TextMaterial_MainMenu_MouseOver.TextMaterial_MainMenu_MouseOver")
    (Class|GameplayStatics|PlaySoundAttached "/Game/Audio/Click_04.Click_04" _text_quit)))

(event OnEndCursorOver(Button_Quit)
  (params (TouchedComponent :type Primitive%20Component%20Object%20Reference))
  ;[1 1 1] Quit Button
  (if (Variables|Default|GetIsActive)
    (Rendering|Material|SetMaterial (Variables|Default|GetText_Quit) 0 "/Game/Materials/TextMaterial_MainMenu.TextMaterial_MainMenu")))

(event OnClicked(Button_Options)
  (params (TouchedComponent :type Primitive%20Component%20Object%20Reference))
  ;[1 1 1] Options Button
  (if (Variables|Default|GetIsActive)
    (Default|CallOptionsButtonClicked)
    (Rendering|Material|SetMaterial (Variables|Default|GetText_Options) 0 "/Game/Materials/TextMaterial_MainMenu.TextMaterial_MainMenu")))

(event OnBeginCursorOver(Button_Options)
  (params (TouchedComponent :type Primitive%20Component%20Object%20Reference))
  (bind _text_options (Variables|Default|GetText_Options))
  ;[1 1 1] Options Button
  (if (Variables|Default|GetIsActive)
    (Rendering|Material|SetMaterial _text_options 0 "/Game/Materials/TextMaterial_MainMenu_MouseOver.TextMaterial_MainMenu_MouseOver")
    (Class|GameplayStatics|PlaySoundAttached "/Game/Audio/Click_04.Click_04" _text_options)))

(event OnEndCursorOver(Button_Options)
  (params (TouchedComponent :type Primitive%20Component%20Object%20Reference))
  ;[1 1 1] Options Button
  (if (Variables|Default|GetIsActive)
    (Rendering|Material|SetMaterial (Variables|Default|GetText_Options) 0 "/Game/Materials/TextMaterial_MainMenu.TextMaterial_MainMenu")))

(event OnClicked(Button_Play)
  (params (TouchedComponent :type Primitive%20Component%20Object%20Reference))
  ;[1 1 1] Play Button
  (if (Variables|Default|GetIsActive)
    (Default|CallPlayButtonClicked)
    (Rendering|Material|SetMaterial (Variables|Default|GetText_Play) 0 "/Game/Materials/TextMaterial_MainMenu.TextMaterial_MainMenu")))

(fn ConstructionScript)