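; PlayMenu is a main-menu Blueprint for the play screen, with Players and Back buttons shown as text components in the world.
; Cursor-over events swap each text's material to a highlight and play an attached click sound, and cursor exit restores the normal material.
; Clicking Players opens the Prototype_Smith level, while the Back click event is empty.
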(event OnClicked(Button_Players)
  (params (TouchedComponent :type Primitive%20Component%20Object%20Reference))
  ;[1 1 1] Players Button
  (Game|OpenLevel(byName) "Prototype_Smith"))

(event OnBeginCursorOver(Button_Players)
  (params (TouchedComponent :type Primitive%20Component%20Object%20Reference))
  (bind _text_players (Variables|Default|GetText_Players))
  ;[1 1 1] Players Button
  (Rendering|Material|SetMaterial _text_players 0 "/Game/Materials/TextMaterial_MainMenu_MouseOver.TextMaterial_MainMenu_MouseOver")
  (Class|GameplayStatics|PlaySoundAttached "/Game/Audio/Click_04.Click_04" _text_players))

(event OnEndCursorOver(Button_Players)
  (params (TouchedComponent :type Primitive%20Component%20Object%20Reference))
  ;[1 1 1] Players Button
  (Rendering|Material|SetMaterial (Variables|Default|GetText_Players) 0 "/Game/Materials/TextMaterial_MainMenu.TextMaterial_MainMenu"))

(event OnClicked(Button_Back)
  (params (TouchedComponent :type Primitive%20Component%20Object%20Reference))
  ;[1 1 1] Back Button
)

(event OnBeginCursorOver(Button_Back)
  (params (TouchedComponent :type Primitive%20Component%20Object%20Reference))
  (bind _text_back (Variables|Default|GetText_Back))
  ;[1 1 1] Back Button
  (Rendering|Material|SetMaterial _text_back 0 "/Game/Materials/TextMaterial_MainMenu_MouseOver.TextMaterial_MainMenu_MouseOver")
  (Class|GameplayStatics|PlaySoundAttached "/Game/Audio/Click_04.Click_04" _text_back))

(event OnEndCursorOver(Button_Back)
  (params (TouchedComponent :type Primitive%20Component%20Object%20Reference))
  ;[1 1 1] Back Button
  (Rendering|Material|SetMaterial (Variables|Default|GetText_Back) 0 "/Game/Materials/TextMaterial_MainMenu.TextMaterial_MainMenu"))

(event EventBeginPlay)

(fn ConstructionScript)