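; Main menu actor with 3D Play, Options and Quit buttons driven by component cursor and click events.
; Hovering a button swaps its text component to a mouse-over material and plays an attached click sound, and leaving restores the normal material.
; Play opens the Prototype_Smith level and Quit exits the game, while the Options click event is empty.
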(event OnClicked(Button_Quit)
  (params (TouchedComponent :type Primitive%20Component%20Object%20Reference))
  ;[1 1 1] Quit Button
  (Game|QuitGame))

(event OnBeginCursorOver(Button_Play)
  (params (TouchedComponent :type Primitive%20Component%20Object%20Reference))
  (bind _text_play (Variables|Default|GetText_Play))
  ;[1 1 1] Play Button
  (Rendering|Material|SetMaterial _text_play 0 "/Game/Materials/TextMaterial_MainMenu_MouseOver.TextMaterial_MainMenu_MouseOver")
  (Class|GameplayStatics|PlaySoundAttached "/Game/Audio/Click_04.Click_04" _text_play))

(event OnEndCursorOver(Button_Play)
  (params (TouchedComponent :type Primitive%20Component%20Object%20Reference))
  ;[1 1 1] Play Button
  (Rendering|Material|SetMaterial (Variables|Default|GetText_Play) 0 "/Game/Materials/TextMaterial_MainMenu.TextMaterial_MainMenu"))

(event OnBeginCursorOver(Button_Quit)
  (params (TouchedComponent :type Primitive%20Component%20Object%20Reference))
  (bind _text_quit (Variables|Default|GetText_Quit))
  ;[1 1 1] Quit Button
  (Rendering|Material|SetMaterial _text_quit 0 "/Game/Materials/TextMaterial_MainMenu_MouseOver.TextMaterial_MainMenu_MouseOver")
  (Class|GameplayStatics|PlaySoundAttached "/Game/Audio/Click_04.Click_04" _text_quit))

(event OnEndCursorOver(Button_Quit)
  (params (TouchedComponent :type Primitive%20Component%20Object%20Reference))
  ;[1 1 1] Quit Button
  (Rendering|Material|SetMaterial (Variables|Default|GetText_Quit) 0 "/Game/Materials/TextMaterial_MainMenu.TextMaterial_MainMenu"))

(event OnClicked(Button_Options)
  (params (TouchedComponent :type Primitive%20Component%20Object%20Reference))
  ;[1 1 1] Options Button
)

(event OnBeginCursorOver(Button_Options)
  (params (TouchedComponent :type Primitive%20Component%20Object%20Reference))
  (bind _text_options (Variables|Default|GetText_Options))
  ;[1 1 1] Options Button
  (Rendering|Material|SetMaterial _text_options 0 "/Game/Materials/TextMaterial_MainMenu_MouseOver.TextMaterial_MainMenu_MouseOver")
  (Class|GameplayStatics|PlaySoundAttached "/Game/Audio/Click_04.Click_04" _text_options))

(event OnEndCursorOver(Button_Options)
  (params (TouchedComponent :type Primitive%20Component%20Object%20Reference))
  ;[1 1 1] Options Button
  (Rendering|Material|SetMaterial (Variables|Default|GetText_Options) 0 "/Game/Materials/TextMaterial_MainMenu.TextMaterial_MainMenu"))

(event OnClicked(Button_Play)
  (params (TouchedComponent :type Primitive%20Component%20Object%20Reference))
  ;[1 1 1] Play Button
  (Game|OpenLevel(byName) "Prototype_Smith"))

(fn ConstructionScript)